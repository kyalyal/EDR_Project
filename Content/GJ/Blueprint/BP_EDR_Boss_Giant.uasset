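; Giant boss enemy Blueprint that handles hit feedback and kill-quest reporting.
; Point damage spawns a large blood burst at the hit location with undead and damage sounds, until HP reaches zero and IsHpZero blocks further feedback.
; Any actor overlap while the Death flag is true reports the kill to the first QuestManager found in the level.
; Death is only read here, never set.
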(event `self.ReceiveActorBeginOverlap`
  (params (OtherActor :type "Actor Object Reference"))
  (if (`self.Death`)
    (bind _outactors (`GameplayStatics.GetAllActorsOfClass` "/Game/JSW/Npc/Quest/QuestManager.QuestManager_C"))
    (`/Game/JSW/Npc/Quest/QuestManager.CheckKillQuest` (`|GetArrayItem` _outactors) 200)))

(event `self.ReceivePointDamage`
  (params (Damage :type "Float (single-precision)") (DamageType :type "DamageType Object Reference") (HitLocation :type "Vector Structure") (HitNormal :type "Vector Structure") (HitComponent :type "PrimitiveComponent Object Reference") (BoneName :type Name) (ShotFromDirection :type "Vector Structure") (InstigatedBy :type "Controller Object Reference") (DamageCauser :type "Actor Object Reference") (HitInfo :type "HitResult Structure (by ref)"))
  (if (not (`self.IsHpZero`))
    (`KismetSystemLibrary.PrintString` "blood")
    (`NiagaraFunctionLibrary.SpawnSystemAtLocation` "/Game/Vefects/Blood_VFX/VFX/VAT_Versions/Bursts/One_Shot/OS_NS_HD_Blood_Burst_Large.OS_NS_HD_Blood_Burst_Large" HitLocation (`KismetMathLibrary.Conv_VectorToRotator` HitLocation) (10.0 10.0 10.0))
    (`GameplayStatics.PlaySoundAtLocation` "/Game/Monster_Sounds_Volume_01/Cues/Undead_02_Cue.Undead_02_Cue" (`self.K2_GetActorLocation`) (struct) 1.0 1.0 0.0 null null null null)
    (`GameplayStatics.PlaySoundAtLocation` "/Game/Sword_Fighting_SFX/Wavs/Damage_Que.Damage_Que" (`self.K2_GetActorLocation`) (struct) 1.0 1.0 0.0 null null null null)
    (if (<= (`self.GetHp`) 0.0)
      (set `self.IsHpZero` true))))

(fn `UserConstructionScript`)