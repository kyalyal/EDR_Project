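; GJ_BP_MyCharacter is an AI-driven melee character that chases and attacks the player once it sees them.
; PawnSensing triggers FollowPlayer, which uses AIMoveTo toward the player, then plays a sword montage and waits out its length.
; The sighting flag then clears, so chasing resumes only on the next sighting.
; Tick and overlap handlers do nothing, and the turn-around patrol logic is disconnected.
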(event `self.ReceiveBeginPlay`)

(event `self.ReceiveTick`
  (params (DeltaSeconds :type "Float (single-precision)"))
  (if (`self.isSeeingPlayer`)
    _))

(event `self.AttackRange.OnComponentBeginOverlap`
  (params (OverlappedComponent :type "PrimitiveComponent Object Reference") (OtherActor :type "Actor Object Reference") (OtherComp :type "PrimitiveComponent Object Reference") (OtherBodyIndex :type Integer) (bFromSweep :type Boolean) (SweepResult :type "HitResult Structure (by ref)")))

(event `self.PawnSensing.OnSeePawn`
  (params (Pawn :type "Pawn Object Reference"))
  (set `self.isSeeingPlayer` true)
  (`self.FollowPlayer` self))

(event `FollowPlayer`
  (set `self.canAttack` true)
  (if (`self.isSeeingPlayer`)
    (`|AIMoveTo` self (0.0 0.0 0.0) (`GameplayStatics.GetPlayerCharacter` 0) 150.0
      (:`OnSuccess`
        (if (`self.canAttack`)
          (set `self.canAttack` false)
          (bind _returnvalue (`self.PlayAnimMontage` "/Game/GJ/Animation/SwordAttack1_Montage.SwordAttack1_Montage"))
          (`KismetSystemLibrary.Delay` _returnvalue)
          (set `self.canAttack` true)
          (set `self.isSeeingPlayer` false))))
    (else
      (set `self.isSeeingPlayer` false))))

(fn `rotateActor180`
  (`self.K2_SetActorRotation` (`KismetMathLibrary.MakeRotator` (.roll (`self.K2_GetActorRotation`)) (.pitch (`self.K2_GetActorRotation`)) (+ (.yaw (`self.K2_GetActorRotation`)) 180.0))))

(fn `UserConstructionScript`)