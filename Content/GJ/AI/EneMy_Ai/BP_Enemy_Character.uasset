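; BP_Enemy_Character is an enemy character with health and attack damage set on BeginPlay.
; An overlap on its AttackRange component subtracts the damage from a MyTestEDRCharacter's Hp and prints the result, then runs a trailing Delay that gates nothing.
; Attack1 plays a sword animation, while Attack2, Attack3 and Pase2 are placeholders that only print debug strings.
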(event `self.ReceiveBeginPlay`
  (set `self.AttackDamage` 10.0)
  (set `self.hp` 60.0))

(event `self.AttackRange.OnComponentBeginOverlap`
  (params (OverlappedComponent :type "PrimitiveComponent Object Reference") (OtherActor :type "Actor Object Reference") (OtherComp :type "PrimitiveComponent Object Reference") (OtherBodyIndex :type Integer) (bFromSweep :type Boolean) (SweepResult :type "HitResult Structure (by ref)"))
  (bind _asmy_test_edrcharacter (cast `/Game/GJ/Blueprint/MyTestEDRCharacter` OtherActor))
  (bind _returnvalue (- (`TestEDRCharacter.hp` _asmy_test_edrcharacter) (`self.AttackDamage`)))
  (`KismetSystemLibrary.PrintString` (`KismetStringLibrary.Conv_DoubleToString` _returnvalue))
  (set `TestEDRCharacter.hp` _returnvalue _asmy_test_edrcharacter)
  (`KismetSystemLibrary.Delay` 2.0))

(fn `Attack 1`
  (`KismetSystemLibrary.PrintString` "NormalAttack")
  (`SkeletalMeshComponent.PlayAnimation` (`self.Mesh`) "/Game/GJ/Animation/Enemy_Anim/SwordAttack_sk.SwordAttack_sk" false))

(fn `Attack2`
  (`KismetSystemLibrary.PrintString` "MiddleAttack"))

(fn `Attack3`
  (`KismetSystemLibrary.PrintString` "Punch"))

(fn `Pase2`
  (`KismetSystemLibrary.PrintString` "Pase 22222"))

(fn `UserConstructionScript`)